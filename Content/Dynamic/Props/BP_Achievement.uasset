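; BP_Achievement is a trophy shelf prop that shows unlocked achievements and their story entries.
; On BeginPlay it loads achievement flags from the SaveScore slot, or defaults all to locked, then toggles shelf and trophy meshes to match.
; Each display entry holds the story when unlocked, otherwise its unlock condition.
; Box overlap sets the Exterminator's indicator, while ShowStory and Exit swap a paused achievement UI with the HUD.
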(event `self.ReceiveBeginPlay`
  ;[1 1 1] Loading save game
  (bind _returnvalue (`GameplayStatics.DoesSaveGameExist` "SaveScore"))
  (if _returnvalue
    (bind _returnvalue_2 (`GameplayStatics.LoadGameFromSlot` "SaveScore"))
    (bind _asbp_user_save_file (cast `/Game/Dynamic/SaveFile/BP_UserSaveFile` _returnvalue_2))
    (set `self.Achievements` (`/Game/Dynamic/SaveFile/BP_UserSaveFile.Achievements Unlocked` _asbp_user_save_file))
    (else
      (set `self.Achievements` (`|MakeArray` false false false false false false false false false false))))
  (`self.Set Stories`)
  (`self.Setting visibility`))

(event `Previous`
  (bind _story_portion (`self.Story Portion`))
  ;[1 1 1] Navigation
  (if (> _story_portion 0)
    (`/Engine/EditorBlueprintResources/StandardMacros.DecrementInt` _story_portion)))

(event `Set Stories`
  ;[1 1 1] Setting display
  (for (_array_element _array_index) (`self.Story`)
    (if (`|GetArrayItem` (`self.Achievements`) _array_index)
      (`KismetArrayLibrary.Array_Insert` (`self.Display`) _array_element _array_index)
      (else
        (`KismetArrayLibrary.Array_Insert` (`self.Display`) (`|GetArrayItem` (`self.Unlock Condition`) _array_index) _array_index)))))

(event `Next`
  (bind _story_portion (`self.Story Portion`))
  ;[1 1 1] Navigation
  (if (< _story_portion 9)
    (`/Engine/EditorBlueprintResources/StandardMacros.IncrementInt` _story_portion)))

(event `Exit`
  (bind _returnvalue (`GameplayStatics.GetPlayerController` 0))
  ;[1 1 1] Exit story viewing
  (set `PlayerController.bShowMouseCursor` false _returnvalue)
  (`GameplayStatics.SetGamePaused` false)
  (`WidgetLayoutLibrary.RemoveAllWidgets`)
  (`WidgetBlueprintLibrary.SetInputMode_GameOnly` _returnvalue)
  (bind _returnvalue_2 (`|CreateWidget` "/Game/Dynamic/UI/HUD/HUD.HUD_C"))
  (`UserWidget.AddToViewport` _returnvalue_2 0))

(event `Show Story`
  (bind _returnvalue (`GameplayStatics.GetPlayerController` 0))
  ;[1 1 1] View story
  (`WidgetLayoutLibrary.RemoveAllWidgets`)
  (bind _returnvalue_2 (`|CreateWidget` "/Game/Dynamic/UI/Achievements/UI_Achievement.UI_Achievement_C"))
  (`UserWidget.AddToViewport` _returnvalue_2 0)
  (set `PlayerController.bShowMouseCursor` true _returnvalue)
  (`WidgetBlueprintLibrary.SetInputMode_UIOnlyEx` _returnvalue _returnvalue_2)
  (`GameplayStatics.SetGamePaused` true))

(event `self.Box.OnComponentBeginOverlap`
  (params (OverlappedComponent :type "PrimitiveComponent Object Reference") (OtherActor :type "Actor Object Reference") (OtherComp :type "PrimitiveComponent Object Reference") (OtherBodyIndex :type Integer) (bFromSweep :type Boolean) (SweepResult :type "HitResult Structure (by ref)"))
  ;[1 1 1] Interaction
  (bind _asbp_exterminator (cast `/Game/Dynamic/Characters/Exterminator/Blueprint/BP_Exterminator` OtherActor))
  (set `ExterminatorMannequin.Indicator` 17 _asbp_exterminator))

(event `self.Box.OnComponentEndOverlap`
  (params (OverlappedComponent :type "PrimitiveComponent Object Reference") (OtherActor :type "Actor Object Reference") (OtherComp :type "PrimitiveComponent Object Reference") (OtherBodyIndex :type Integer))
  ;[1 1 1] Interaction
  (bind _asbp_exterminator (cast `/Game/Dynamic/Characters/Exterminator/Blueprint/BP_Exterminator` OtherActor))
  (set `ExterminatorMannequin.Indicator` 0 _asbp_exterminator))

(fn `Setting visibility`
  (bind _achievements (`self.Achievements`))
  (bind _output (`|GetArrayItem` _achievements))
  (`SceneComponent.SetVisibility` (`self.Shelf bottom`) _output false)
  (`SceneComponent.SetVisibility` (`self.Shelf`) _output false)
  (`SceneComponent.SetVisibility` (`self.Shelf top`) _output false)
  (`SceneComponent.SetVisibility` (`self.StaticMeshComponent`) (`|GetArrayItem` _achievements 1) false)
  (`SceneComponent.SetVisibility` (`self.Trophy 2`) (`|GetArrayItem` _achievements 2) false)
  (`SceneComponent.SetVisibility` (`self.Trophy 3`) (`|GetArrayItem` _achievements 3) false)
  (`SceneComponent.SetVisibility` (`self.Trophy 4`) (`|GetArrayItem` _achievements 4) false)
  (`SceneComponent.SetVisibility` (`self.Trophy 5`) (`|GetArrayItem` _achievements 5) false)
  (`SceneComponent.SetVisibility` (`self.Trophy 6`) (`|GetArrayItem` _achievements 6) false)
  (`SceneComponent.SetVisibility` (`self.Trophy 7`) (`|GetArrayItem` _achievements 7) false)
  (`SceneComponent.SetVisibility` (`self.Trophy 8`) (`|GetArrayItem` _achievements 8) false)
  (`SceneComponent.SetVisibility` (`self.Trophy 9`) (`|GetArrayItem` _achievements 9) false))

(fn `UserConstructionScript`)