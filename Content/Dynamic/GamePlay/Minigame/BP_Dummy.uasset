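; BP_Dummy is a hittable target for a minigame that awards points when struck.
; On a component hit it tips over 90 degrees, disables collision and adds ScorePerHit to the first BP_Minigame found in the level.
; After ResetTime it rotates back up and re-enables collision, but stays down if the minigame cast fails.
; The construction script applies the Material variable to the dummy mesh.
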(event `self.Dummy.OnComponentHit`
  (params (HitComponent :type "PrimitiveComponent Object Reference") (OtherActor :type "Actor Object Reference") (OtherComp :type "PrimitiveComponent Object Reference") (NormalImpulse :type "Vector Structure") (Hit :type "HitResult Structure (by ref)"))
  (`SceneComponent.K2_AddLocalRotation` (`self.Dummy`) (struct :`Roll` 90.0) false false)
  (`PrimitiveComponent.SetCollisionEnabled` (`self.Dummy`) "NoCollision")
  (bind _outactors (`GameplayStatics.GetAllActorsOfClass` "/Game/Dynamic/GamePlay/Minigame/BP_Minigame.BP_Minigame_C"))
  (bind _asbp_minigame (cast `/Game/Dynamic/GamePlay/Minigame/BP_Minigame` (`|GetArrayItem` _outactors))
    (:`then`
      (`/Game/Dynamic/GamePlay/Minigame/BP_Minigame.Increase Score` _asbp_minigame (`self.Score per Hit`))
      (`KismetSystemLibrary.PrintString` "Hit")
      (`KismetSystemLibrary.Delay` (`self.Reset Time`))
      (`SceneComponent.K2_AddLocalRotation` (`self.Dummy`) (struct :`Roll` -90.0) false false)
      (`KismetSystemLibrary.PrintString` "Rotated Back")
      (`PrimitiveComponent.SetCollisionEnabled` (`self.Dummy`) "QueryAndPhysics"))
    (:`CastFailed`
      (`KismetSystemLibrary.PrintString` "Cast Failed" true true (struct :`R` 1.0 :`B` 0.968458 :`A` 1.0)))))

(fn `UserConstructionScript`
  (`PrimitiveComponent.SetMaterial` (`self.Dummy`) 0 (`self.Material`)))