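; BP_Graphics is a world prop through which the player opens a graphics settings menu.
; Its box overlap sets the BP_Exterminator's Indicator, and enter/exit events swap HUD and UI_Settings widgets, toggling pause, cursor and input mode.
; Low to Epic presets, or custom values derived by ChangeValues from one float, feed SetNewGraphicsSettings, which applies resolution scale and scalability levels through GameUserSettings.
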(event `self.ReceiveBeginPlay`
  ;[1 1 1] Initialization
  (bind _asbp_exterminator (cast `/Game/Dynamic/Characters/Exterminator/Blueprint/BP_Exterminator` (`GameplayStatics.GetPlayerPawn` 0)))
  (set `self.Player Reference` _asbp_exterminator))

(event `Epic`
  ;[1 1 1] Preset settings
  (`self.Set New Graphics Settings` 100.0 3))

(event `High`
  ;[1 1 1] Preset settings
  (`self.Set New Graphics Settings` 75.0 2))

(event `self.Box.OnComponentBeginOverlap`
  (params (OverlappedComponent :type "PrimitiveComponent Object Reference") (OtherActor :type "Actor Object Reference") (OtherComp :type "PrimitiveComponent Object Reference") (OtherBodyIndex :type Integer) (bFromSweep :type Boolean) (SweepResult :type "HitResult Structure (by ref)"))
  ;[1 1 1] Overlap event
  (bind _asbp_exterminator (cast `/Game/Dynamic/Characters/Exterminator/Blueprint/BP_Exterminator` OtherActor))
  (set `ExterminatorMannequin.Indicator` 12 _asbp_exterminator))

(event `Custom Graphics Settings`
  ;[1 1 1] Custom Graphics settings
  (`self.Set New Graphics Settings` (`self.Float Value`) (`self.Integer Value`)))

(event `Medium`
  ;[1 1 1] Preset settings
  (`self.Set New Graphics Settings` 50.0 1))

(event `self.Box.OnComponentEndOverlap`
  (params (OverlappedComponent :type "PrimitiveComponent Object Reference") (OtherActor :type "Actor Object Reference") (OtherComp :type "PrimitiveComponent Object Reference") (OtherBodyIndex :type Integer))
  ;[1 1 1] Overlap event
  (bind _asbp_exterminator (cast `/Game/Dynamic/Characters/Exterminator/Blueprint/BP_Exterminator` OtherActor))
  (set `ExterminatorMannequin.Indicator` 0 _asbp_exterminator))

(event `Low`
  ;[1 1 1] Preset settings
  (`self.Set New Graphics Settings` 25.0))

(event `Exit Graphic Menu`
  (bind _returnvalue (`GameplayStatics.GetPlayerController` 0))
  ;[1 1 1] Exit from Graphics Menu
  (set `/Game/Dynamic/Characters/Exterminator/Blueprint/BP_Exterminator.PressF` false (`self.Player Reference`))
  (set `PlayerController.bShowMouseCursor` false _returnvalue)
  (`GameplayStatics.SetGamePaused` false)
  (`WidgetLayoutLibrary.RemoveAllWidgets`)
  (`WidgetBlueprintLibrary.SetInputMode_GameOnly` _returnvalue)
  (bind _returnvalue_2 (`|CreateWidget` "/Game/Dynamic/UI/HUD/HUD.HUD_C"))
  (`UserWidget.AddToViewport` _returnvalue_2 0))

(event `Enter Graphics Menu`
  (bind _returnvalue (`GameplayStatics.GetPlayerController` 0))
  ;[1 1 1] Enter Into Graphics Menu]
  (`WidgetLayoutLibrary.RemoveAllWidgets`)
  (bind _returnvalue_2 (`|CreateWidget` "/Game/Dynamic/UI/GraphicsMenu/UI_Settings.UI_Settings_C"))
  (`UserWidget.AddToViewport` _returnvalue_2 0)
  (set `PlayerController.bShowMouseCursor` true _returnvalue)
  (`WidgetBlueprintLibrary.SetInputMode_UIOnlyEx` _returnvalue _returnvalue_2)
  (`GameplayStatics.SetGamePaused` true))

(fn `Change Values`
  (params (Float :type "Float (double-precision)"))
  (bind _returnvalue (* 100 Float))
  (set `self.Float Value` _returnvalue)
  (set `self.Integer Value` (`KismetMathLibrary.FTrunc` (- (/ _returnvalue 4.0) 1.0))))

(fn `Set New Graphics Settings`
  (params (NewScaleValue :type "Float (double-precision)") (InputPin :type Integer))
  (bind _returnvalue (`GameUserSettings.GetGameUserSettings`))
  (`GameUserSettings.SetAntiAliasingQuality` _returnvalue InputPin)
  (`GameUserSettings.SetTextureQuality` _returnvalue InputPin)
  (`GameUserSettings.SetPostProcessingQuality` _returnvalue InputPin)
  (`GameUserSettings.SetResolutionScaleValueEx` _returnvalue NewScaleValue)
  (`GameUserSettings.SetFoliageQuality` _returnvalue InputPin)
  (`GameUserSettings.SetViewDistanceQuality` _returnvalue InputPin)
  (`GameUserSettings.SetShadowQuality` _returnvalue InputPin)
  (`GameUserSettings.SetVisualEffectQuality` _returnvalue InputPin)
  (`GameUserSettings.ApplySettings` _returnvalue false))

(fn `UserConstructionScript`)