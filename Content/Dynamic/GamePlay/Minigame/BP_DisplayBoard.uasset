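; BP_DisplayBoard is a minigame display board that shows a text message for a limited time.
; Its ShowText event stores the given text and duration, sets the TextRender component's text and makes it visible.
; After a Delay of that duration it hides the component and its children again.
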(event `Show Text`
  (params (Text :type String) (Duration :type "Float (double-precision)"))
  (set `self.Text` Text)
  (set `self.Duration` Duration)
  (`TextRenderComponent.K2_SetText` (`self.TextRender`) (`KismetTextLibrary.Conv_StringToText` (`self.Text`)))
  (`SceneComponent.SetVisibility` (`self.TextRender`) true true)
  (`KismetSystemLibrary.Delay` (`self.Duration`))
  (`SceneComponent.SetVisibility` (`self.TextRender`) false true))

(fn `UserConstructionScript`)