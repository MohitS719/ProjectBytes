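; BP_RiggedDoor is a door prop that snaps open once when something overlaps its Box1 trigger.
; A separate Box trigger shows its TextRender on begin overlap and hides it on end overlap.
; Box1 passes through a DoOnce, sets the door's relative rotation instantly with no animation, and plays an open/close sound at the player pawn's location.
; Neither trigger filters the overlapping actor.
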(event `self.Box.OnComponentBeginOverlap`
  (params (OverlappedComponent :type "PrimitiveComponent Object Reference") (OtherActor :type "Actor Object Reference") (OtherComp :type "PrimitiveComponent Object Reference") (OtherBodyIndex :type Integer) (bFromSweep :type Boolean) (SweepResult :type "HitResult Structure (by ref)"))
  (`SceneComponent.SetVisibility` (`self.TextRender`) true true))

(event `self.Box1.OnComponentBeginOverlap`
  (params (OverlappedComponent :type "PrimitiveComponent Object Reference") (OtherActor :type "Actor Object Reference") (OtherComp :type "PrimitiveComponent Object Reference") (OtherBodyIndex :type Integer) (bFromSweep :type Boolean) (SweepResult :type "HitResult Structure (by ref)"))
  (`/Engine/EditorBlueprintResources/StandardMacros.DoOnce` false
    (:`Completed`
      (`SceneComponent.K2_SetRelativeRotation` (`self.Door`) (struct :`Yaw` -90.0) false false)
      (`GameplayStatics.PlaySoundAtLocation` "/Game/Static/Sound/Door_OpenClose_Cue.Door_OpenClose_Cue" (`self.K2_GetActorLocation` (`GameplayStatics.GetPlayerPawn` 0))))))

(event `self.Box.OnComponentEndOverlap`
  (params (OverlappedComponent :type "PrimitiveComponent Object Reference") (OtherActor :type "Actor Object Reference") (OtherComp :type "PrimitiveComponent Object Reference") (OtherBodyIndex :type Integer))
  (`SceneComponent.SetVisibility` (`self.TextRender`) false true))

(fn `UserConstructionScript`)