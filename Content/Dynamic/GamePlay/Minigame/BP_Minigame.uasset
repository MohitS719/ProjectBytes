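; Timed score minigame actor that the player starts with F inside its trigger box, with an indicator light showing when it runs.
; F runs a countdown on BP_DisplayBoard, then opens a timed window in which IncreaseScore calls add points.
; At the end it shows the score, inserts it into a top-five array and saves that through Bytes_SAVE.
; BP_ScoreBoard, taken as the second actor found, refreshes on load and after each round.
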(event `self.Box.OnComponentBeginOverlap`
  (params (OverlappedComponent :type "PrimitiveComponent Object Reference") (OtherActor :type "Actor Object Reference") (OtherComp :type "PrimitiveComponent Object Reference") (OtherBodyIndex :type Integer) (bFromSweep :type Boolean) (SweepResult :type "HitResult Structure (by ref)"))
  ;[1 1 1] Switch Input Mechanism
  (if (not (`self.Enabled`))
    (`self.EnableInput` (`GameplayStatics.GetPlayerController` 0))))

(event `self.Box.OnComponentEndOverlap`
  (params (OverlappedComponent :type "PrimitiveComponent Object Reference") (OtherActor :type "Actor Object Reference") (OtherComp :type "PrimitiveComponent Object Reference") (OtherBodyIndex :type Integer))
  ;[1 1 1] Switch Input Mechanism
  (`self.DisableInput` (`GameplayStatics.GetPlayerController` 0)))

(event `Key|F`
  (params (Key :type "Key Structure"))
  ;[1 1 1] Main
  (:`Pressed`
    (`self.DisableInput` (`GameplayStatics.GetPlayerController` 0))
    (`LightComponent.SetLightColor` (`self.Indicator`) (`self.On Color`) true)
    (set `self.Score` 0)
    (bind _outactors (`GameplayStatics.GetAllActorsOfClass` "/Game/Dynamic/GamePlay/Minigame/BP_DisplayBoard.BP_DisplayBoard_C"))
    (bind _asbp_display_board (cast `/Game/Dynamic/GamePlay/Minigame/BP_DisplayBoard` (`|GetArrayItem` _outactors)))
    (`/Game/Dynamic/GamePlay/Minigame/BP_DisplayBoard.Show Text` _asbp_display_board "Get Ready" 1.5)
    (`KismetSystemLibrary.Delay` 1.6)
    (`/Game/Dynamic/GamePlay/Minigame/BP_DisplayBoard.Show Text` _asbp_display_board "Set" 1.5)
    (`KismetSystemLibrary.Delay` 1.6)
    (`/Game/Dynamic/GamePlay/Minigame/BP_DisplayBoard.Show Text` _asbp_display_board "GO!!!" 0.6)
    (set `self.Enabled` true)
    (`KismetSystemLibrary.PrintString` "Game On")
    (`KismetSystemLibrary.Delay` (`self.Duration`))
    (`KismetSystemLibrary.PrintString` "Game End")
    (set `self.Enabled` false)
    (`KismetSystemLibrary.PrintString` (`KismetStringLibrary.Conv_IntToString` (`self.Score`)) true true (struct :`R` 1.0 :`G` 0.101284 :`A` 1.0) 8.0)
    (`LightComponent.SetLightColor` (`self.Indicator`) (`self.Off Color`) true)
    (`/Game/Dynamic/GamePlay/Minigame/BP_DisplayBoard.Show Text` _asbp_display_board (`KismetStringLibrary.Concat_StrStr` (`self.Score Text`) (`KismetStringLibrary.Conv_IntToString` (`self.Score`))) 5.0)
    (`self.Calculate Score`)
    (bind _asbytes_save (cast `/Game/Dynamic/SaveFile/Bytes_SAVE` (`self.Save Game Sub`)))
    (set `/Game/Dynamic/SaveFile/Bytes_SAVE.Minigame Scores` (`self.Score Array`) _asbytes_save)
    (`GameplayStatics.SaveGameToSlot` (`self.Save Game Sub`) "Slot1")
    (`self.Refresh Scores`)))

(event `Increase Score`
  (params (`Added Score` :type Integer))
  ;[1 1 1] Score Increment
  (if (`self.Enabled`)
    (set `self.Score` (+ `Added Score` (`self.Score`)))
    (`KismetSystemLibrary.PrintString` "Score Increased" true true (struct :`R` 1.0 :`G` 0.793835 :`A` 1.0))
    (else
      (`KismetSystemLibrary.PrintString` "Game not ON" true true (struct :`G` 1.0 :`B` 0.065727 :`A` 1.0)))))

(event `self.ReceiveBeginPlay`
  ;[1 0.3116 0.804] Loading save game on begin play
  (bind _returnvalue (`GameplayStatics.DoesSaveGameExist` "Slot1"))
  (if _returnvalue
    (bind _returnvalue_2 (`GameplayStatics.LoadGameFromSlot` "Slot1"))
    (bind _output_get (set `self.Save Game Sub` _returnvalue_2))
    (bind _asbytes_save (cast `/Game/Dynamic/SaveFile/Bytes_SAVE` _output_get))
    (set `self.Score Array` (`/Game/Dynamic/SaveFile/Bytes_SAVE.Minigame Scores` _asbytes_save))
    (else
      (bind _returnvalue_3 (`GameplayStatics.CreateSaveGameObject` "/Game/Dynamic/SaveFile/Bytes_SAVE.Bytes_SAVE_C"))
      (bind _output_get_2 (set `self.Save Game Sub` _returnvalue_3))
      (bind _asbytes_save_2 (cast `/Game/Dynamic/SaveFile/Bytes_SAVE` _output_get_2))
      (set `self.Score Array` (`/Game/Dynamic/SaveFile/Bytes_SAVE.Minigame Scores` _asbytes_save_2))))
  (`self.Refresh Scores`)
  (`KismetSystemLibrary.PrintString` "Save Game Loading Complete" true true (struct :`R` 1.0 :`G` 0.209691 :`B` 0.716425 :`A` 1.0)))

(event `Key|P`
  (params (Key :type "Key Structure"))
  ;[1 0 0.02813] Debug
  (:`Pressed`
    (for _array_element (`self.Score Array`)
      (`KismetSystemLibrary.PrintString` (`KismetStringLibrary.Conv_IntToString` _array_element) true true (struct :`R` 1.0 :`G` 0.940401 :`A` 1.0) 8.0))))

(fn `Calculate Score`
  (bind _score (`self.Score`))
  ;[0 0.3786 1] Sorts and Places Score
  (for _index (range 5)
    (if (> _score (`|GetArrayItem` (`self.Score Array`) _index))
      (`KismetArrayLibrary.Array_Insert` (`self.Score Array`) _score _index)
      (`KismetArrayLibrary.Array_Resize` (`self.Score Array`) 5)
      (break))))

(fn `Refresh Scores`
  (bind _score_array (`self.Score Array`))
  (bind _outactors (`GameplayStatics.GetAllActorsOfClass` "/Game/Dynamic/GamePlay/Minigame/BP_ScoreBoard.BP_ScoreBoard_C"))
  (bind _asbp_score_board (cast `/Game/Dynamic/GamePlay/Minigame/BP_ScoreBoard` (`|GetArrayItem` _outactors 1)))
  (`/Game/Dynamic/GamePlay/Minigame/BP_ScoreBoard.Update Score` _asbp_score_board (`|GetArrayItem` _score_array) (`|GetArrayItem` _score_array 1) (`|GetArrayItem` _score_array 2) (`|GetArrayItem` _score_array 3) (`|GetArrayItem` _score_array 4)))

(fn `UserConstructionScript`
  (`LightComponent.SetLightColor` (`self.Indicator`) (`self.Off Color`) true))