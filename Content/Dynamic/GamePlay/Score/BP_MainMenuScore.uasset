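; BP_MainMenuScore is an actor that fills the main menu scoreboard with the player's best five scores.
; On BeginPlay it loads the BP_UserSaveFile save from its slot, or creates a new save object if none exists, and copies BestFiveScores into ScoreArray.
; UpdateScore then finds the first BP_ScoreBoard actor in the level and passes it the five values.
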(event `self.ReceiveBeginPlay`
  (bind _slot_name (`self.Slot name`))
  (bind _user_index (`self.User Index`))
  (bind _returnvalue (`GameplayStatics.DoesSaveGameExist` _slot_name _user_index))
  (if _returnvalue
    (bind _returnvalue_2 (`GameplayStatics.LoadGameFromSlot` _slot_name _user_index))
    (bind _output_get (set `self.Save Game Sub` _returnvalue_2))
    (bind _asbp_user_save_file (cast `/Game/Dynamic/SaveFile/BP_UserSaveFile` _output_get))
    (set `self.Score Array` (`/Game/Dynamic/SaveFile/BP_UserSaveFile.Best Five Scores` _asbp_user_save_file))
    (else
      (bind _returnvalue_3 (`GameplayStatics.CreateSaveGameObject` "/Game/Dynamic/SaveFile/BP_UserSaveFile.BP_UserSaveFile_C"))
      (bind _output_get_2 (set `self.Save Game Sub` _returnvalue_3))
      (bind _asbp_user_save_file_2 (cast `/Game/Dynamic/SaveFile/BP_UserSaveFile` _output_get_2))
      (set `self.Score Array` (`/Game/Dynamic/SaveFile/BP_UserSaveFile.Best Five Scores` _asbp_user_save_file_2))))
  (`self.Update Score`))

(fn `Update Score`
  (bind _score_array (`self.Score Array`))
  (bind _outactors (`GameplayStatics.GetAllActorsOfClass` "/Game/Dynamic/GamePlay/Minigame/BP_ScoreBoard.BP_ScoreBoard_C"))
  (bind _asbp_score_board (cast `/Game/Dynamic/GamePlay/Minigame/BP_ScoreBoard` (`|GetArrayItem` _outactors)))
  (`/Game/Dynamic/GamePlay/Minigame/BP_ScoreBoard.Update Score` _asbp_score_board (`|GetArrayItem` _score_array) (`|GetArrayItem` _score_array 1) (`|GetArrayItem` _score_array 2) (`|GetArrayItem` _score_array 3) (`|GetArrayItem` _score_array 4)))

(fn `UserConstructionScript`)