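; Loot box prop that a BP_Exterminator opens with a keycard to drop pickups.
; Box overlap registers the box with the player and toggles a world-space prompt.
; OpenBox calls the player's UseKeycard, animates lid and lock, and rolls weighted drops at nine spawners, mostly health or ammo, rarely power-ups.
; After a delay it closes into a timed lockdown, shown as red "Locked" text until a function-name timer resets it.
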(event `Reset Lock down`
  ;[1 1 1] Unlock
  (set `self.Lockdown` false)
  (`KismetSystemLibrary.K2_SetTimer` "/Game/Dynamic/Pickups/BP_KeyCard.BP_KeyCard" "Reset Lock down")
  (set `self.Text` "Press F To Unlock")
  (set `self.Text Color` (`KismetMathLibrary.Conv_LinearColorToColor` (`KismetMathLibrary.MakeColor` 0.0 255.0)))
  (`self.Render Text`))

(event `self.ReceiveBeginPlay`
  ;[1 1 1] Initializing Spawner Array
  (set `self.Spawners` (`|MakeArray` (`self.SpawnerFive`) (`self.SpawnerTwo`) (`self.SpawnerThree`) (`self.SpawnerFour`) (`self.Spawner`) (`self.SpawnerSix`) (`self.SpawnerSeven`) (`self.SpawnerEight`) (`self.SpawnerNine`) :!type "SceneComponent Object Reference"))
  (`self.Render Text`))

(event `self.Box.OnComponentBeginOverlap`
  (params (OverlappedComponent :type "PrimitiveComponent Object Reference") (OtherActor :type "Actor Object Reference") (OtherComp :type "PrimitiveComponent Object Reference") (OtherBodyIndex :type Integer) (bFromSweep :type Boolean) (SweepResult :type "HitResult Structure (by ref)"))
  ;[1 0.9646 0.604] Input Mechanism
  (bind _asbp_exterminator (cast `/Game/Dynamic/Characters/Exterminator/Blueprint/BP_Exterminator` OtherActor))
  (set `ExterminatorMannequin.Indicator` 18 _asbp_exterminator)
  (set `/Game/Dynamic/Characters/Exterminator/Blueprint/BP_Exterminator.Loot Box Reference` self _asbp_exterminator)
  (if (not (`self.Opened`))
    (`SceneComponent.SetVisibility` (`self.TextRender`) true true)))

(event `self.Box.OnComponentEndOverlap`
  (params (OverlappedComponent :type "PrimitiveComponent Object Reference") (OtherActor :type "Actor Object Reference") (OtherComp :type "PrimitiveComponent Object Reference") (OtherBodyIndex :type Integer))
  ;[1 0.9646 0.604] Input Mechanism
  (bind _asbp_exterminator (cast `/Game/Dynamic/Characters/Exterminator/Blueprint/BP_Exterminator` OtherActor))
  (set `ExterminatorMannequin.Indicator` 0 _asbp_exterminator)
  (`SceneComponent.SetVisibility` (`self.TextRender`) false true))

(event `Open Box`
  ;[1 0.6966 0.8131] Main Flow
  (if (not (`self.Opened`))
    (bind _keycard (`self.Does player Have Keycard`))
    (if (and _keycard (not (`self.Lockdown`)))
      (set `self.Opened` true)
      (`SceneComponent.SetVisibility` (`self.TextRender`) false true)
      (`SceneComponent.K2_AddRelativeRotation` (`self.LootBox_Lid`) (struct :`Roll` -120.0) false false)
      (`SceneComponent.K2_SetRelativeLocation` (`self.LootBox_Lock`) (0.0 0.0 35.0) false false)
      (for _array_element (`self.Spawners`)
        (`self.Spawn Pickup` _array_element (`KismetMathLibrary.RandomIntegerInRange` 0 99)))
      (`KismetSystemLibrary.Delay` (`self.Opened Duration`))
      (`SceneComponent.K2_AddRelativeRotation` (`self.LootBox_Lid`) (struct :`Roll` 120.0) false false)
      (`SceneComponent.K2_SetRelativeLocation` (`self.LootBox_Lock`) (0.0 0.0 45.0) false false)
      (set `self.Opened` false)
      (set `self.Lockdown` true)
      (`KismetSystemLibrary.K2_SetTimer` self "Reset Lock down" 25.0)
      (set `self.Text` "Locked")
      (set `self.Text Color` (`KismetMathLibrary.Conv_LinearColorToColor` (`KismetMathLibrary.MakeColor` 255.0)))
      (`self.Render Text`))))

(fn `Does player Have Keycard`
  (returns (KeyCard :type Boolean))
  (bind _outactors (`GameplayStatics.GetAllActorsOfClass` "/Game/Dynamic/Characters/Exterminator/Blueprint/BP_Exterminator.BP_Exterminator_C"))
  (bind _asbp_exterminator (cast `/Game/Dynamic/Characters/Exterminator/Blueprint/BP_Exterminator` (`|GetArrayItem` _outactors)))
  (bind _output_get (set `self.Player Reference` _asbp_exterminator))
  (bind _returnvalue (`ExterminatorMannequin.UseKeycard` _output_get))
  (return _returnvalue))

(fn `Render Text`
  (`TextRenderComponent.K2_SetText` (`self.TextRender`) (`self.Text`))
  (`TextRenderComponent.SetTextRenderColor` (`self.TextRender`) (`self.Text Color`))
  (`TextRenderComponent.SetWorldSize` (`self.TextRender`) (`self.Text Size`))
  (`TextRenderComponent.SetFont` (`self.TextRender`) (`self.Font`)))

(fn `Spawn Pickup`
  (params (Spawner :type "SceneComponent Object Reference") (Chances :type Integer))
  (if (and (> Chances 0) (<= Chances 44))
    ;[1 1 1] Health Drop 45%
    (`|SpawnActorFromClass` "/Game/Dynamic/Pickups/BP_HealthPickUp.BP_HealthPickUp_C" (`SceneComponent.K2_GetComponentToWorld` Spawner) "AlwaysSpawn" "OverrideRootScale" null null)
    (elif (and (> Chances 44) (<= Chances 90))
      ;[1 1 1] Ammo Drop 45%
      (`|SpawnActorFromClass` "/Game/Dynamic/Pickups/BP_AmmoPickUp.BP_AmmoPickUp_C" (`SceneComponent.K2_GetComponentToWorld` Spawner) "AdjustIfPossibleButAlwaysSpawn" "OverrideRootScale" null null)
      (elif (and (> Chances 90) (<= Chances 94))
        ;[1 1 1] Invincibility Drop 4%
        (`|SpawnActorFromClass` "/Game/Dynamic/Pickups/BP_Invincibility.BP_Invincibility_C" (`SceneComponent.K2_GetComponentToWorld` Spawner) "AlwaysSpawn" "OverrideRootScale" null null)
        (elif (and (> Chances 94) (<= Chances 98))
          ;[1 1 1] One Shot kill Drop 4%
          (`|SpawnActorFromClass` "/Game/Dynamic/Pickups/BP_OneShotKill.BP_OneShotKill_C" (`SceneComponent.K2_GetComponentToWorld` Spawner) "AlwaysSpawn" "OverrideRootScale" null null)
          (elif (>= Chances 98)
            ;[1 1 1] Kill All Drop 1%
            (`|SpawnActorFromClass` "/Game/Dynamic/Pickups/BP_KillAll.BP_KillAll_C" (`SceneComponent.K2_GetComponentToWorld` Spawner) "AlwaysSpawn" "OverrideRootScale" null null)))))))

(fn `UserConstructionScript`)