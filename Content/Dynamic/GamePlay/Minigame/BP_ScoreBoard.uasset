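; Minigame scoreboard actor that displays a title and five numbered score rows using text render components.
; The construction script sets the title text and applies the shared font, plus separate color and size settings for the title and the rows.
; The UpdateScore event receives five integer scores and writes them to the P1–P5 texts as given, with no sorting or storage.
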(event `Update Score`
  (params (P1 :type Integer) (P2 :type Integer) (P3 :type Integer) (P4 :type Integer) (P5 :type Integer))
  (`TextRenderComponent.K2_SetText` (`self.P1`) (`KismetTextLibrary.Conv_IntToText` P1))
  (`TextRenderComponent.K2_SetText` (`self.P2`) (`KismetTextLibrary.Conv_IntToText` P2))
  (`TextRenderComponent.K2_SetText` (`self.P3`) (`KismetTextLibrary.Conv_IntToText` P3))
  (`TextRenderComponent.K2_SetText` (`self.P4`) (`KismetTextLibrary.Conv_IntToText` P4))
  (`TextRenderComponent.K2_SetText` (`self.P5`) (`KismetTextLibrary.Conv_IntToText` P5)))

(fn `UserConstructionScript`
  (bind _font (`self.Font`))
  (bind _score_color (`self.Score Color`))
  (bind _score_size (`self.Score Size`))
  (`TextRenderComponent.K2_SetText` (`self.Title`) (`self.Title Text`))
  (`TextRenderComponent.SetFont` (`self.No1`) _font)
  (`TextRenderComponent.SetFont` (`self.No2`) _font)
  (`TextRenderComponent.SetFont` (`self.No3`) _font)
  (`TextRenderComponent.SetFont` (`self.No4`) _font)
  (`TextRenderComponent.SetFont` (`self.No5`) _font)
  (`TextRenderComponent.SetFont` (`self.P1`) _font)
  (`TextRenderComponent.SetFont` (`self.P2`) _font)
  (`TextRenderComponent.SetFont` (`self.P3`) _font)
  (`TextRenderComponent.SetFont` (`self.P4`) _font)
  (`TextRenderComponent.SetFont` (`self.P5`) _font)
  (`TextRenderComponent.SetFont` (`self.Title`) _font)
  (`TextRenderComponent.SetTextRenderColor` (`self.Title`) (`self.Title Color`))
  (`TextRenderComponent.SetTextRenderColor` (`self.P5`) _score_color)
  (`TextRenderComponent.SetTextRenderColor` (`self.P4`) _score_color)
  (`TextRenderComponent.SetTextRenderColor` (`self.P3`) _score_color)
  (`TextRenderComponent.SetTextRenderColor` (`self.P2`) _score_color)
  (`TextRenderComponent.SetTextRenderColor` (`self.P1`) _score_color)
  (`TextRenderComponent.SetTextRenderColor` (`self.No5`) _score_color)
  (`TextRenderComponent.SetTextRenderColor` (`self.No4`) _score_color)
  (`TextRenderComponent.SetTextRenderColor` (`self.No3`) _score_color)
  (`TextRenderComponent.SetTextRenderColor` (`self.No2`) _score_color)
  (`TextRenderComponent.SetTextRenderColor` (`self.No1`) _score_color)
  (`TextRenderComponent.SetWorldSize` (`self.No1`) _score_size)
  (`TextRenderComponent.SetWorldSize` (`self.No2`) _score_size)
  (`TextRenderComponent.SetWorldSize` (`self.No3`) _score_size)
  (`TextRenderComponent.SetWorldSize` (`self.No4`) _score_size)
  (`TextRenderComponent.SetWorldSize` (`self.No5`) _score_size)
  (`TextRenderComponent.SetWorldSize` (`self.P1`) _score_size)
  (`TextRenderComponent.SetWorldSize` (`self.P2`) _score_size)
  (`TextRenderComponent.SetWorldSize` (`self.P3`) _score_size)
  (`TextRenderComponent.SetWorldSize` (`self.P4`) _score_size)
  (`TextRenderComponent.SetWorldSize` (`self.P5`) _score_size)
  (`TextRenderComponent.SetWorldSize` (`self.Title`) (`self.Title Size`)))