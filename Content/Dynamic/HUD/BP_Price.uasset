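; BP_Price stores the current prices for five purchases: ammo capacity, damage and health capacity upgrades, plus health and ammo refills.
; BeginPlay sets the starting prices, with refills cheaper than upgrades.
; One function per item raises its price by a fixed step, larger for upgrades than for refills.
; It only tracks prices, with no purchase, currency or display logic.
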(event `self.ReceiveBeginPlay`
  (set `self.Ammo Capacity Price` 5)
  (set `self.Damage Price` 5)
  (set `self.Health Capacity Price` 5)
  (set `self.Refill Health Price` 3)
  (set `self.Refill Ammo Price` 3))

(fn `Increase Ammo Capacity Price`
  (set `self.Ammo Capacity Price` (+ (`self.Ammo Capacity Price`) 10)))

(fn `Increase Damage Price`
  (set `self.Damage Price` (+ (`self.Damage Price`) 10)))

(fn `Increase Health Capacity Price`
  (set `self.Health Capacity Price` (+ (`self.Health Capacity Price`) 10)))

(fn `Increase Refill Ammo Price`
  (set `self.Refill Ammo Price` (+ (`self.Refill Ammo Price`) 2)))

(fn `Increase Refill Health Price`
  (set `self.Refill Health Price` (+ (`self.Refill Health Price`) 2)))

(fn `UserConstructionScript`)