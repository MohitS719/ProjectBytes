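; Flickering light prop that is active while a BP_Exterminator overlaps its trigger box.
; On begin overlap it opens a Gate and starts a loop that sets a random stepped intensity on the point light, plays a flicker sound, then re-enters the Gate after a random delay.
; On end overlap it closes the Gate, sets intensity to zero and plays the sound once more with randomized volume and pitch.
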(event `self.Trigger Box.OnComponentBeginOverlap`
  (params (OverlappedComponent :type "PrimitiveComponent Object Reference") (OtherActor :type "Actor Object Reference") (OtherComp :type "PrimitiveComponent Object Reference") (OtherBodyIndex :type Integer) (bFromSweep :type Boolean) (SweepResult :type "HitResult Structure (by ref)"))
  (cast `/Game/Dynamic/Characters/Exterminator/Blueprint/BP_Exterminator` OtherActor)
  (`|ExecutionSequence`
    (:`then_0`
      (goto _label_2 :!via `Open`))
    (:`then_1`
      (`LightComponent.SetIntensity` (`self.PointLight`) (`KismetMathLibrary.Conv_IntToDouble` (* (`KismetMathLibrary.RandomIntegerInRange` 0 3) 50)) :!label _label)
      (`|ExecutionSequence`
        (:`then_0`
          (`KismetSystemLibrary.Delay` (`KismetMathLibrary.RandomFloatInRange` 1.0 2.0))
          (`/Engine/EditorBlueprintResources/StandardMacros.Gate` true :!label _label_2
            (:`Exit`
              (goto _label))))
        (:`then_1`
          (`GameplayStatics.PlaySoundAtLocation` "/Game/Static/Maps/CustomContent/Audio/LightFlicker_Cue.LightFlicker_Cue" (`SceneComponent.K2_GetComponentLocation` (`self.PointLight`)) (struct) (`KismetMathLibrary.RandomFloatInRange` 0.2 0.6) (`KismetMathLibrary.RandomFloatInRange` 0.95 1.05) :!label _label_3))))))

(event `self.Trigger Box.OnComponentEndOverlap`
  (params (OverlappedComponent :type "PrimitiveComponent Object Reference") (OtherActor :type "Actor Object Reference") (OtherComp :type "PrimitiveComponent Object Reference") (OtherBodyIndex :type Integer))
  (cast `/Game/Dynamic/Characters/Exterminator/Blueprint/BP_Exterminator` OtherActor)
  (`|ExecutionSequence`
    (:`then_0`
      (goto _label_2 :!via `Close`))
    (:`then_1`
      (`LightComponent.SetIntensity` (`self.PointLight`) 0.0)
      (goto _label_3))))

(fn `UserConstructionScript`)