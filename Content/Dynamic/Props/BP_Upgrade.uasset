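; BP_Upgrade is an upgrade machine whose trigger sets the Exterminator's PressF flag while the player is in range.
; BeginPlay caches the character, shotgun and pistol upgrade scene actors.
; Each menu event shows its widget, spawns a new camera at that scene's CameraSpawnPosition, switches the view and enables UI-only input.
; Exiting restores game input and the HUD, then calls BackToRealWorld on the Exterminator.
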(event `Go To Shotgun Upgrade Menu`
  ;[1 1 1] Character Upgrade Portion
  (set `self.InUpgradeMachine` true)
  (`WidgetLayoutLibrary.RemoveAllWidgets`)
  (bind _returnvalue (`|CreateWidget` "/Game/Dynamic/UI/UpgradeMachine/ShotgunUpgrade.ShotgunUpgrade_C"))
  (`self.Create Upgrade Menu` _returnvalue (`SceneComponent.K2_GetComponentToWorld` (`/Game/Dynamic/Props/ShotgunUpgradeScene.Camera Spawn Position` (`self.Shotgun Upgrade Scene`)))))

(event `self.ReceiveBeginPlay`
  ;[1 1 1] Initialization
  (`self.Get Character Upgrade Scene`)
  (`self.Get Shotgun upgrade Scene`)
  (`self.Get Pistol Upgrate Scene`))

(event `self.Trigger.OnComponentBeginOverlap`
  (params (OverlappedComponent :type "PrimitiveComponent Object Reference") (OtherActor :type "Actor Object Reference") (OtherComp :type "PrimitiveComponent Object Reference") (OtherBodyIndex :type Integer) (bFromSweep :type Boolean) (SweepResult :type "HitResult Structure (by ref)"))
  ;[1 1 1] Overlap event
  (bind _asbp_exterminator (cast `/Game/Dynamic/Characters/Exterminator/Blueprint/BP_Exterminator` OtherActor))
  (set `/Game/Dynamic/Characters/Exterminator/Blueprint/BP_Exterminator.PressF` true _asbp_exterminator))

(event `Go To Character Upgrade Menu`
  ;[1 1 1] Shotgun Upgrade Portion
  (set `self.InUpgradeMachine` true)
  (`WidgetLayoutLibrary.RemoveAllWidgets`)
  (bind _returnvalue (`|CreateWidget` "/Game/Dynamic/UI/UpgradeMachine/CharacterUpgrade.CharacterUpgrade_C"))
  (`self.Create Upgrade Menu` _returnvalue (`SceneComponent.K2_GetComponentToWorld` (`/Game/Dynamic/Props/CharacterUpgradeScene.Camera Spawn Position` (`self.Character Upgrade Scene`)))))

(event `self.Trigger.OnComponentEndOverlap`
  (params (OverlappedComponent :type "PrimitiveComponent Object Reference") (OtherActor :type "Actor Object Reference") (OtherComp :type "PrimitiveComponent Object Reference") (OtherBodyIndex :type Integer))
  ;[1 1 1] Overlap event
  (bind _asbp_exterminator (cast `/Game/Dynamic/Characters/Exterminator/Blueprint/BP_Exterminator` OtherActor))
  (set `/Game/Dynamic/Characters/Exterminator/Blueprint/BP_Exterminator.PressF` false _asbp_exterminator))

(event `Go To Pistol Upgrade Menu`
  ;[1 1 1] Pistol Upgrade Portion
  (set `self.InUpgradeMachine` true)
  (`WidgetLayoutLibrary.RemoveAllWidgets`)
  (bind _returnvalue (`|CreateWidget` "/Game/Dynamic/UI/UpgradeMachine/PistolUpgrade.PistolUpgrade_C"))
  (`self.Create Upgrade Menu` _returnvalue (`SceneComponent.K2_GetComponentToWorld` (`/Game/Dynamic/Props/PistolUpgradeScene.Camera Spawn Position` (`self.Pistol Upgrade Scene`)))))

(event `Exit Upgrade Machine`
  ;[1 1 1] Back to game
  (set `self.InUpgradeMachine` false)
  (`KismetSystemLibrary.Delay` 0.2)
  (set `PlayerController.bShowMouseCursor` false (`GameplayStatics.GetPlayerController` 0))
  (`GameplayStatics.SetGamePaused` false)
  (`WidgetLayoutLibrary.RemoveAllWidgets`)
  (`WidgetBlueprintLibrary.SetInputMode_GameOnly` (`GameplayStatics.GetPlayerController` 0))
  (bind _returnvalue (`|CreateWidget` "/Game/Dynamic/UI/HUD/HUD.HUD_C"))
  (`UserWidget.AddToViewport` _returnvalue 0)
  (bind _asbp_exterminator (cast `/Game/Dynamic/Characters/Exterminator/Blueprint/BP_Exterminator` (`GameplayStatics.GetPlayerPawn` 0)))
  (`/Game/Dynamic/Characters/Exterminator/Blueprint/BP_Exterminator.Back to Real World` _asbp_exterminator))

(fn `Create Upgrade Menu`
  (params (`Upgrade Widget` :type "UserWidget Object Reference") (SpawnTransform :type "Transform Structure"))
  (bind _returnvalue (`GameplayStatics.GetPlayerController` 0))
  (`UserWidget.AddToViewport` `Upgrade Widget` 0)
  (bind _returnvalue_2 (`|SpawnActorFromClass` "/Script/Engine.CameraActor" SpawnTransform "Undefined" "OverrideRootScale" null null))
  (`PlayerController.SetViewTargetWithBlend` _returnvalue _returnvalue_2 0.0 "VTBlend_EaseIn" 0.0 false)
  (set `PlayerController.bShowMouseCursor` true _returnvalue)
  (`WidgetBlueprintLibrary.SetInputMode_UIOnlyEx` _returnvalue)
  (`GameplayStatics.SetGamePaused` false))

(fn `Get Character Upgrade Scene`
  (bind _outactors (`GameplayStatics.GetAllActorsOfClass` "/Game/Dynamic/Props/CharacterUpgradeScene.CharacterUpgradeScene_C"))
  (bind _ascharacter_upgrade_scene (cast `/Game/Dynamic/Props/CharacterUpgradeScene` (`|GetArrayItem` _outactors)))
  (set `self.Character Upgrade Scene` _ascharacter_upgrade_scene))

(fn `Get Pistol Upgrate Scene`
  (bind _outactors (`GameplayStatics.GetAllActorsOfClass` "/Game/Dynamic/Props/PistolUpgradeScene.PistolUpgradeScene_C"))
  (bind _aspistol_upgrade_scene (cast `/Game/Dynamic/Props/PistolUpgradeScene` (`|GetArrayItem` _outactors)))
  (set `self.Pistol Upgrade Scene` _aspistol_upgrade_scene))

(fn `Get Shotgun upgrade Scene`
  (bind _outactors (`GameplayStatics.GetAllActorsOfClass` "/Game/Dynamic/Props/ShotgunUpgradeScene.ShotgunUpgradeScene_C"))
  (bind _asshotgun_upgrade_scene (cast `/Game/Dynamic/Props/ShotgunUpgradeScene` (`|GetArrayItem` _outactors)))
  (set `self.Shotgun Upgrade Scene` _asshotgun_upgrade_scene))

(fn `UserConstructionScript`)