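; BP_Proximity_Light is a prop light that turns on only while something overlaps its trigger box.
; The construction script applies exposed intensity, attenuation radius and color to the PointLight and starts it hidden.
; Box begin and end overlap events toggle the light's visibility, with no filtering on the overlapping actor or count of overlaps.
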(event `self.Box.OnComponentBeginOverlap`
  (params (OverlappedComponent :type "PrimitiveComponent Object Reference") (OtherActor :type "Actor Object Reference") (OtherComp :type "PrimitiveComponent Object Reference") (OtherBodyIndex :type Integer) (bFromSweep :type Boolean) (SweepResult :type "HitResult Structure (by ref)"))
  (`SceneComponent.SetVisibility` (`self.PointLight`) true false))

(event `self.Box.OnComponentEndOverlap`
  (params (OverlappedComponent :type "PrimitiveComponent Object Reference") (OtherActor :type "Actor Object Reference") (OtherComp :type "PrimitiveComponent Object Reference") (OtherBodyIndex :type Integer))
  (`SceneComponent.SetVisibility` (`self.PointLight`) false false))

(fn `UserConstructionScript`
  (`LightComponent.SetIntensity` (`self.PointLight`) (`self.Intensity`))
  (`PointLightComponent.SetAttenuationRadius` (`self.PointLight`) (`self.Attenuation Radius`))
  (`LightComponent.SetLightColor` (`self.PointLight`) (`self.Light Color`) true)
  (`SceneComponent.SetVisibility` (`self.PointLight`) false false))