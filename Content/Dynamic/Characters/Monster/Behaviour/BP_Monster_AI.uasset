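; BP_Monster_AI is an AI controller that drives a BP_Exterminator pawn through patrol and combat.
; On BeginPlay it sets up the BB_PatrolData blackboard and runs the BT_GaurdBehaviour tree.
; Perception updates set or clear the enemy blackboard key, while Tick switches the pawn's aiming and shooting on whenever a focus actor exists.
; FindPatrolRoute, not called in this graph, writes the pawn's first patrol point to WayPoint.
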(event `self.ReceiveTick`
  (params (DeltaSeconds :type "Float (single-precision)"))
  ;[1 1 1] Setting AI to aim iron sight when enemy is in focus
  (bind _asbp_exterminator (cast `/Game/Dynamic/Characters/Exterminator/Blueprint/BP_Exterminator` (`self.K2_GetPawn`)))
  (bind _output_get (set `/Game/Dynamic/Characters/Exterminator/Blueprint/BP_Exterminator.Aiming` (`KismetSystemLibrary.IsValid` (`self.GetFocusActor`)) _asbp_exterminator))
  (set `/Game/Dynamic/Characters/Exterminator/Blueprint/BP_Exterminator.Shooting` _output_get _asbp_exterminator))

(event `self.ReceiveBeginPlay`
  ;[1 1 1] Set Focal Point
  (bind _blackboardcomponent (`self.UseBlackboard` "/Game/Dynamic/Characters/Exterminator/Behaviour/BB_PatrolData.BB_PatrolData"))
  (`self.RunBehaviorTree` "/Game/Dynamic/Characters/Exterminator/Behaviour/BT_GaurdBehaviour.BT_GaurdBehaviour")
  (set `self.BlackboardComp` _blackboardcomponent))

(event `self.AIPerception.OnTargetPerceptionUpdated`
  (params (Actor :type "Actor Object Reference") (Stimulus :type "AIStimulus Structure"))
  (bind _blackboardcomp (`self.BlackboardComp`))
  (bind _enemykey (`self.EnemyKey`))
  (if (`.bSuccessfullySensed` (break `AIStimulus` Stimulus))
    (`BlackboardComponent.SetValueAsObject` _blackboardcomp _enemykey Actor)
    (else
      (`BlackboardComponent.ClearValue` _blackboardcomp _enemykey))))

(fn `Find Patrol Route`
  (params (Blackboard :type "BlackboardComponent Object Reference"))
  (bind _asbp_exterminator (cast `/Game/Dynamic/Characters/Exterminator/Blueprint/BP_Exterminator` (`self.K2_GetPawn`)))
  (`BlackboardComponent.SetValueAsObject` Blackboard "WayPoint" (`|GetArrayItem` (`/Game/Dynamic/Characters/Exterminator/Blueprint/BP_Exterminator.PatrolPoints` _asbp_exterminator))))

(fn `UserConstructionScript`)