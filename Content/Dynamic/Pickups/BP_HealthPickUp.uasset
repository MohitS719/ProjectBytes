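; Health pickup that restores a small random amount of health when a BP_Exterminator overlaps its HealthLogo component.
; The character's Heal result decides the outcome: success plays a pickup sound and destroys the actor, while failure plays an error sound and clears DisplayHealthFull after a short delay.
; A BeginPlay timer calls Disappear after a minute, which also clears that flag and removes the pickup.
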(event `self.HealthLogo.OnComponentBeginOverlap`
  (params (OverlappedComponent :type "PrimitiveComponent Object Reference") (OtherActor :type "Actor Object Reference") (OtherComp :type "PrimitiveComponent Object Reference") (OtherBodyIndex :type Integer) (bFromSweep :type Boolean) (SweepResult :type "HitResult Structure (by ref)"))
  (bind _asbp_exterminator (cast `/Game/Dynamic/Characters/Exterminator/Blueprint/BP_Exterminator` OtherActor))
  (bind _returnvalue (`ExterminatorMannequin.Heal` _asbp_exterminator (`KismetMathLibrary.Conv_IntToDouble` (`KismetMathLibrary.RandomIntegerInRange` 5 15))))
  (if _returnvalue
    (bind _returnvalue_2 (`self.K2_GetActorLocation` _asbp_exterminator))
    ;[1 1 1] Successfully Healed
    (`GameplayStatics.PlaySoundAtLocation` "/Game/Static/PickUps/Health/SC_Health_Pickup.SC_Health_Pickup" _returnvalue_2)
    (`self.K2_DestroyActor`)
    (else
      ;[1 1 1] Failed to heal
      (`GameplayStatics.PlaySoundAtLocation` "/Game/Static/Sound/S_Failure2_Cue.S_Failure2_Cue" _returnvalue_2)
      (`KismetSystemLibrary.Delay` 2.0)
      (set `ExterminatorMannequin.bDisplayHealthFull` false _asbp_exterminator))))

(event `Disappear`
  ;[1 1 1] Making Pick Up Disappear
  (set `ExterminatorMannequin.bDisplayHealthFull` false (stale `self.HealthLogo.OnComponentBeginOverlap` _asbp_exterminator))
  (`self.K2_DestroyActor`))

(event `self.ReceiveBeginPlay`
  ;[1 1 1] Setting Up Timer
  (`KismetSystemLibrary.K2_SetTimer` self "Disappear" 60.0))

(fn `UserConstructionScript`)